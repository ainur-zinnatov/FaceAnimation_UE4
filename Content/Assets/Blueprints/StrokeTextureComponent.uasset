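; StrokeTextureComponent draws strokes onto a render target and exposes the result as a texture.
; DrawLine opens a canvas on the target, draws one colored line of given thickness and closes it, while Clear fills the target with a color.
; GetTexture converts the render target to a UTexture2D through a helper that its comment attributes to the TensorFlow library.
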(fn `Clear`
  (params (ClearColor :type "LinearColor Structure"))
  (`KismetRenderingLibrary.ClearRenderTarget2D` (`self.TextureRender`) ClearColor))

(fn `DrawLine`
  (params (From :type "Vector2D Structure") (To :type "Vector2D Structure") (Color :type "LinearColor Structure") (Thickness :type "Float (double-precision)" :default 1.0))
  (bind (_canvas _size _context) (`KismetRenderingLibrary.BeginDrawCanvasToRenderTarget` (`self.TextureRender`)))
  (`Canvas.K2_DrawLine` _canvas From To Thickness Color)
  (`KismetRenderingLibrary.EndDrawCanvasToRenderTarget` _context))

(fn `GetTexture`
  (returns (Texture :type "Texture2D Object Reference"))
  (return (`TensorFlowBlueprintLibrary.Conv_RenderTargetTextureToTexture2D` (`self.TextureRender`))))