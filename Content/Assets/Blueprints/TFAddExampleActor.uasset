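; Example actor that demonstrates talking to a TensorFlow Python script through a TensorflowComponent.
; Pressing F sends ExampleStruct as JSON input and shows it on a text render, and the returned results are written to a second text render.
; Pressing G alternates between minus and plus by calling the script's changeOperation custom function through a ChangeOperation helper.
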(event `Key|F`
  (params (Key :type "Key Structure"))
  (bind _returnvalue (`SIOJsonObject.EncodeJson` (`SIOJLibrary.StructToJsonObject` (`self.ExampleStruct`))))
  (:`Pressed`
    (`/TensorFlow/TensorflowComponent.SendJsonInput` (`self.TensorflowComponent`) _returnvalue) ; send the struct as json input
    (`TextRenderComponent.K2_SetText` (`self.Sent Text`) (`KismetTextLibrary.Conv_StringToText` (`KismetStringLibrary.Concat_StrStr` "Sent: " _returnvalue))) ; update our sent text render
  ))

(event `Key|G`
  (params (Key :type "Key Structure"))
  (:`Pressed`
    (`/Engine/EditorBlueprintResources/StandardMacros.FlipFlop`
      (:`A`
        (`self.ChangeOperation` "-") ; class function to keep bp clean, open to see custom function call
      )
      (:`B`
        (`self.ChangeOperation` "+")))))

(event `self.TensorflowComponent.OnInputResults`
  (params (Results :type String))
  (`TextRenderComponent.K2_SetText` (`self.Result Text`) (`KismetTextLibrary.Conv_StringToText` Results)))

(fn `ChangeOperation`
  (params (NewOperation :type String))
  (`/TensorFlow/TensorflowComponent.CallCustomFunction` (`self.TensorflowComponent`) "changeOperation" NewOperation)
  (`TextRenderComponent.K2_SetText` (`self.Result Text`) (`KismetTextLibrary.Conv_StringToText` (`KismetStringLibrary.Concat_StrStr` "Operation changed to " NewOperation))))

(fn `UserConstructionScript`)